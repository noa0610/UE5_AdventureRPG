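; NPC Blueprint that the player can talk to, with dialogue that changes according to game flags.
; It creates a hidden WBP_ActionGuide widget on BeginPlay and shows it while BP_Belt_4way overlaps its Capsule.
; BPITalkStart walks SearchTalkEventRow through DT_TalkEvent, stopping at the first row whose required flag is unset or on in BP_GameInstance.
; It returns that row's lines, branches and flags; an older row-search path is left unused.
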(event OnComponentBeginOverlap(Capsule)
  (params (OverlappedComponent :type Primitive%20Component%20Object%20Reference) (OtherActor :type Actor%20Object%20Reference) (OtherComp :type Primitive%20Component%20Object%20Reference) (OtherBodyIndex :type Integer) (bFromSweep :type Boolean) (SweepResult :type Hit%20Result%20Structure%20%28by%20ref%29))
  ;[0.15 0.15 0.15 0.5] アクションガイドの表示切り替え
  (Utilities|Casting|CastToBP_Belt_4way OtherActor)
  (Widget|SetVisibility (Variables|Default|GetActionGuide) "Visible") ; 表示
)

(event OnComponentEndOverlap(Capsule)
  (params (OverlappedComponent :type Primitive%20Component%20Object%20Reference) (OtherActor :type Actor%20Object%20Reference) (OtherComp :type Primitive%20Component%20Object%20Reference) (OtherBodyIndex :type Integer))
  ;[0.15 0.15 0.15 0.5] アクションガイドの表示切り替え
  (Utilities|Casting|CastToBP_Belt_4way OtherActor)
  (Widget|SetVisibility (Variables|Default|GetActionGuide) "Hidden") ; 非表示
)

(event Custom|Search_TalkData
  (Utilities|GetDataTableRow "/Game/TPSprite/Blueprints/Event/DT_TalkEvent.DT_TalkEvent" (Utilities|String|StringToName (Utilities|String|ToString(Integer) (Variables|Default|GetSearch_TalkRow)))))

(event EventBeginPlay
  (bind _returnvalue (UserInterface|CreateWidget "/Game/TPSprite/Blueprints/Event/WBP_ActionGuide.WBP_ActionGuide_C")) ; アクションガイド用ウィジェット作成
  (UserInterface|Viewport|AddtoViewport _returnvalue 0)
  (bind _output_get (Variables|Default|SetActionGuide _returnvalue))
  (Widget|SetVisibility _output_get "Hidden") ; 切り替えるまで非表示
)

(event Collision|EventActorBeginOverlap
  (params (OtherActor :type Actor%20Object%20Reference)))

(event EventBPITalkEnd
  (params (WBP_Talk :type WBP%20Talk%20Object%20Reference) (Talking :type Boolean) (NPC :type BP%20NPC%20Belt%20Object%20Reference) (SetFlag :type E_Flag%20Enum :default "NewEnumerator2")))

(event EventTick
  (params (DeltaSeconds :type Float%20%28single-precision%29)))

(fn ConstructionScript)

(fn BPITalkStart
  (params (WBP_Talk :type WBP%20Talk%20Object%20Reference) (Talking :type Boolean) (NPC :type BP%20NPC%20Belt%20Object%20Reference))
  (bind _array_element (Utilities|Array|ForEachLoopwithBreak (Variables|Default|GetSearch_TalkEventRow) :!label _label) ; 昇順でTalkEventを探す
    (:LoopBody
      (bind _returnvalue (Utilities|GetDataTableRow "/Game/TPSprite/Blueprints/Event/DT_TalkEvent.DT_TalkEvent" _array_element)
        (:then
          (if (Utilities|Enum|Equal(Enum) (.requiredflag _returnvalue) "NewEnumerator2") ; None（未設定）の場合はフラグチェックをスルー
            (goto _label Break)
            (else
              (bind _asbp_game_instance (Utilities|Casting|CastToBP_GameInstance (Game|GetGameInstance)))
              (bind _flagchack (Default|FlagChack _asbp_game_instance (.requiredflag _returnvalue)))
              (if _flagchack ; フラグがONのデータを見つけた
                (goto _label Break)))))))
    (:Completed
      (return (.requiredflag _returnvalue) (.setflag _returnvalue) (.talklines _returnvalue) (.branches _returnvalue)))))