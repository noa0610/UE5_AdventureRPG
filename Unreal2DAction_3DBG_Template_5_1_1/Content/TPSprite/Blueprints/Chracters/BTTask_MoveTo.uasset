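; A behavior tree task that moves a BP_Belt_AI_Doge pawn toward a blackboard location.
; Each AI tick it issues a MoveToLocation to the target key's vector and calls the pawn's InputDirection.
; It finishes successfully once the pawn is within a short distance of the player character, measured against the player rather than the blackboard target.
; It also prints the player character's name every tick.
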(event EventReceiveExecuteAI
  (params (OwnerController :type AI%20Controller%20Object%20Reference) (ControlledPawn :type Pawn%20Object%20Reference)))

(event EventReceiveTickAI
  (params (OwnerController :type AI%20Controller%20Object%20Reference) (ControlledPawn :type Pawn%20Object%20Reference) (DeltaSeconds :type Float%20%28single-precision%29))
  (bind _returnvalue (Game|GetPlayerCharacter 0))
  (bind _asbp_belt_ai_doge (Utilities|Casting|CastToBP_Belt_AI_Doge ControlledPawn))
  (Development|PrintString (Utilities|GetDisplayName _returnvalue))
  (AI|Navigation|MovetoLocation OwnerController (Class|BTFunctionLibrary|GetBlackboardValueasVector (Variables|Default|GetTargetBlackboardKey)) 5e+01 true true false true 0)
  (Default|InputDirection _asbp_belt_ai_doge) ; 動かしたい処理
  (if (< (Math|Vector|Distance(Vector) (Transformation|GetActorLocation _returnvalue) (Transformation|GetActorLocation ControlledPawn)) 1.5e+02)
    (AI|BehaviorTree|FinishExecute true)))