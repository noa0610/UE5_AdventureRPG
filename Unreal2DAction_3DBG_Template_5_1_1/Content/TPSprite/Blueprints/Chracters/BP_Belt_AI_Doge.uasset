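; BP_Belt_AI_Doge is a sprite character that animates a Doge from its own movement, with no AI decision logic in this graph.
; Each Tick derives walk, run, jump and fall flags from velocity, then sets the flipbook for that state and one of four facings.
; While moving horizontally, it then splits the velocity angle into eight sectors, updating facing only on cardinals, so diagonals keep the last facing, with debug prints.
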(event Custom|OnCharacterMovementUpdated_Event
  (params (DeltaSeconds :type Float%20%28single-precision%29) (OldLocation :type Vector) (OldVelocity :type Vector)))

(event EventBeginPlay)

(event Collision|EventActorBeginOverlap
  (params (OtherActor :type Actor%20Object%20Reference)))

(event EventTick
  (params (DeltaSeconds :type Float%20%28single-precision%29))
  ;[1 1 0] Tick
  (CallFunction|MovementSetUp)
  (CallFunction|UpdateFlipbook)
  (if (> (Math|Vector|VectorLength (Class|KismetMathLibrary|VectorNormal2D (Transformation|GetVelocity) 0.0001)) 0.0)
    (CallFunction|InputDirection)))

(event EventOnJumped)

(fn ConstructionScript)

(fn UpdateFlipbook
  ;[1 1 1] ActionAnimSet
  ;;[0.15 0.15 0.15 0.5] 状態をAnimSetに保持
  (if (Variables|Character|GetbFall)
    (Variables|Character|SetAnimSet 4)
    (elif (Variables|Character|GetbJump)
      (Variables|Character|SetAnimSet 3)
      (elif (Variables|Character|GetbRun)
        (Variables|Character|SetAnimSet 2)
        (elif (Variables|Character|GetbWalk)
          (Variables|Character|SetAnimSet 1)
          (else
            (Variables|Character|SetAnimSet 0))))))
  ;[0.15 0.15 0.15 0.5] 現在の向きに合わせてアニメーション切り替え
  (switch int (Variables|Character|GetTPSprite_Direction)
    (:0
      ;[1 1 1] Right
      (Sprite|SetFlipbook (Variables|Default|GetSprite) (Utilities|Select :Index (Variables|Character|GetAnimSet) :Option%200 (Variables|キャラクター|GetSprite_000_Idle) :Option%201 (Variables|キャラクター|GetSprite_001_Walk) :Option%202 (Variables|キャラクター|GetSprite_002_Run) :Option%203 (Variables|キャラクター|GetSprite_003_Jump) :Option%204 (Variables|キャラクター|GetSprite_004_Fall))))
    (:1
      ;[1 1 1] Front
      (Sprite|SetFlipbook (Variables|Default|GetSprite) (Utilities|Select :Index (Variables|Character|GetAnimSet) :Option%200 (Variables|キャラクター|GetSprite_200_Idle) :Option%201 (Variables|キャラクター|GetSprite_201_Walk) :Option%202 (Variables|キャラクター|GetSprite_202_Run) :Option%203 (Variables|キャラクター|GetSprite_203_Jump) :Option%204 (Variables|キャラクター|GetSprite_204_Fall))))
    (:2
      ;[1 1 1] Left
      (Sprite|SetFlipbook (Variables|Default|GetSprite) (Utilities|Select :Index (Variables|Character|GetAnimSet) :Option%200 (Variables|キャラクター|GetSprite_400_Idle) :Option%201 (Variables|キャラクター|GetSprie_401_Walk) :Option%202 (Variables|キャラクター|GetSprite_402_Run) :Option%203 (Variables|キャラクター|GetSprite_403_Jump) :Option%204 (Variables|キャラクター|GetSprite_404_Fall))))
    (:3
      ;[1 1 1] Back
      (Sprite|SetFlipbook (Variables|Default|GetSprite) (Utilities|Select :Index (Variables|Character|GetAnimSet) :Option%200 (Variables|キャラクター|GetSprite_600_Idle) :Option%201 (Variables|キャラクター|GetSprite_601_Walk) :Option%202 (Variables|キャラクター|GetSprite_602_Run) :Option%203 (Variables|キャラクター|GetSprite_603_Jump) :Option%204 (Variables|キャラクター|GetSprite_604_Fall))))))

(fn MovementSetUp
  (bind _returnvalue (Transformation|GetVelocity))
  (bind _returnvalue_2 (Math|Vector|VectorLengthXY _returnvalue))
  (Utilities|FlowControl|Sequence
    (:then_0
      ;[1 1 1] Walking Running Set
      (Variables|Character|SetbWalk (> _returnvalue_2 0.0))
      (Variables|Character|SetbRun (> _returnvalue_2 7e+02)))
    (:then_1
      ;[1 1 1] Jumpping Falling Set
      (bind _output_get (Variables|Character|SetbJump (AI|Components|NavMovement|IsFalling (Variables|Character|GetCharacterMovement))))
      (Variables|Character|SetbFall (and _output_get (< (.z (Transformation|GetVelocity)) 0.0))))))

(fn InputDirection
  (bind _returnvalue (Transformation|GetVelocity))
  (bind _returnvalue_2 (Class|KismetMathLibrary|DegAtan2 (.y _returnvalue) (.x _returnvalue)))
  (bind _returnvalue_3 (+ _returnvalue_2 3.6e+02))
  (bind _returnvalue_4 (Math|Float|%(Float) _returnvalue_3 3.6e+02))
  (bind _returnvalue_5 (+ _returnvalue_4 22.5))
  (bind _returnvalue_6 (/ _returnvalue_5 45.0))
  (bind _returnvalue_7 (Math|Float|Floor _returnvalue_6))
  (bind _returnvalue_8 (Math|Integer|%(Integer) _returnvalue_7 8))
  (Development|PrintString (Utilities|String|ToString(Integer) _returnvalue_8))
  (switch int _returnvalue_8 ; 0…右\n1…右上\n2…上\n3…左上\n4…左\n5…左下\n6…下\n7…右下
    (:0
      (Development|PrintString "Right")
      (Variables|Character|SetTPSprite_Direction 0) ; Right
    )
    (:2
      (Development|PrintString "Front")
      (Variables|Character|SetTPSprite_Direction 1) ; Front
    )
    (:4
      (Development|PrintString "Left")
      (Variables|Character|SetTPSprite_Direction 2) ; Left
    )
    (:6
      (Development|PrintString "Back")
      (Variables|Character|SetTPSprite_Direction 3) ; Back
    )))