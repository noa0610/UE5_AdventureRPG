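; NPC Blueprint for a belt quest requester, built on a parent talk-capable NPC class.
; Its talk-start interface override calls the parent with Talking forced false, passing through the parent's name and dialogue text while supplying its own ChackFlag and RewardFlag as the required and set flags.
; The talk-end event is empty, and leftover talk-data search and message nodes in the event graph never run.
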(event EventBeginPlay
  (|CallParentFunction) ; This node is disabled and will not be called.\nDrag off pins to build functionality.
)

(event Collision|EventActorBeginOverlap
  (params (OtherActor :type Actor%20Object%20Reference))
  (|CallParentFunction OtherActor) ; This node is disabled and will not be called.\nDrag off pins to build functionality.
)

(event EventTick
  (params (DeltaSeconds :type Float%20%28single-precision%29))
  (|CallParentFunction DeltaSeconds) ; This node is disabled and will not be called.\nDrag off pins to build functionality.
)

(event EventBPITalkEnd
  (params (WBP_Talk :type WBP%20Talk%20Object%20Reference) (Talking :type Boolean) (NPC :type BP%20NPC%20Belt%20Object%20Reference) (SetFlag :type E_Flag%20Enum :default "NewEnumerator2")))

(fn ConstructionScript
  (|CallParentFunction))

(fn BPITalkStart
  (params (WBP_Talk :type WBP%20Talk%20Object%20Reference) (Talking :type Boolean) (NPC :type BP%20NPC%20Belt%20Object%20Reference))
  (bind (_requiredflag _setflag _nametext _talktext) (|CallParentFunction WBP_Talk false NPC))
  (return (Variables|Default|GetChackFlag) (Variables|Default|GetRewardFlag) _nametext _talktext 0 ""))