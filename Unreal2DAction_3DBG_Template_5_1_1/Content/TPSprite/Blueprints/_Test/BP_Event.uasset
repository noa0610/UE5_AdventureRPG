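; Test event-trigger actor that fires a one-time opening event when the player enters its Sphere collision.
; On overlap by the player character, it asks BP_GameInstance whether a fixed enum flag is already on.
; If not, it prints an opening-event start message as a stand-in and turns on the flag held in its Flag variable.
; The check uses the literal enum value rather than that variable.
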(event OnComponentBeginOverlap(Sphere)
  (params (OverlappedComponent :type Primitive%20Component%20Object%20Reference) (OtherActor :type Actor%20Object%20Reference) (OtherComp :type Primitive%20Component%20Object%20Reference) (OtherBodyIndex :type Integer) (bFromSweep :type Boolean) (SweepResult :type Hit%20Result%20Structure%20%28by%20ref%29))
  (if (== OtherActor (Game|GetPlayerCharacter 0))
    (bind _flagchack (Default|FlagChack (.AsBP%20Game%20Instance (Utilities|Casting|CastToBP_GameInstance (Game|GetGameInstance))) "NewEnumerator0")) ; フラグをチェックする
    (if (not _flagchack)
      (Development|PrintString "オープニングイベント開始" true true "(R=0.000000,G=0.660000,B=1.000000,A=1.000000)" 1e+01)
      (Default|Flagon (.AsBP%20Game%20Instance (Utilities|Casting|CastToBP_GameInstance (Game|GetGameInstance))) (Variables|Default|GetFlag)) ; フラグをONにする
    )))

(event EventBeginPlay)

(event Collision|EventActorBeginOverlap
  (params (OtherActor :type Actor%20Object%20Reference)))

(event EventTick
  (params (DeltaSeconds :type Float%20%28single-precision%29)))

(fn ConstructionScript)