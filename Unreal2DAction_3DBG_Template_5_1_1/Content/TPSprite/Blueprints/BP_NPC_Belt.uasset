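; BP_NPC_Belt is a talkable NPC that shows an action guide and supplies dialogue from a data table.
; It creates a hidden guide widget on BeginPlay, visible only while BP_Belt_4way overlaps its capsule.
; On the talk-start interface event, it recursively steps through numbered DT_TalkData rows until one is talkable or missing.
; A talkable row's name and text go to the talk widget; the talk-end event is empty.
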(event OnComponentBeginOverlap(Capsule)
  (params (OverlappedComponent :type Primitive%20Component%20Object%20Reference) (OtherActor :type Actor%20Object%20Reference) (OtherComp :type Primitive%20Component%20Object%20Reference) (OtherBodyIndex :type Integer) (bFromSweep :type Boolean) (SweepResult :type Hit%20Result%20Structure%20%28by%20ref%29))
  (Utilities|Casting|CastToBP_Belt_4way OtherActor)
  (Widget|SetVisibility (Variables|Default|GetActionGuide) "Visible"))

(event OnComponentEndOverlap(Capsule)
  (params (OverlappedComponent :type Primitive%20Component%20Object%20Reference) (OtherActor :type Actor%20Object%20Reference) (OtherComp :type Primitive%20Component%20Object%20Reference) (OtherBodyIndex :type Integer))
  (Utilities|Casting|CastToBP_Belt_4way OtherActor)
  (Widget|SetVisibility (Variables|Default|GetActionGuide) "Hidden"))

(event Custom|Search_TalkData
  (bind _wbp_talk (Variables|Default|GetWBP%20Talk))
  (bind _returnvalue (Utilities|GetDataTableRow "/Game/TPSprite/Blueprints/DT_TalkData.DT_TalkData" (Utilities|String|StringToName (Utilities|String|ToString(Integer) (Variables|Default|GetSearch_TalkRow))))
    (:then
      (if (.canbetalked _returnvalue)
        (Variables|Default|SetName%20Text (.nametext _returnvalue))
        (Variables|Default|SetTalk%20Text (.talktext _returnvalue))
        (Class|BPIInteract|BPITalkStart(Message) _wbp_talk _wbp_talk false (Variables|Default|GetName%20Text) (Variables|Default|GetTalk%20Text) self "NewEnumerator3" "NewEnumerator3")
        (else
          (bind _result (Math|Integer|IncrementInt (Variables|Default|GetSearch_TalkRow))
            (:%20%20
              (Variables|Default|SetSearch_TalkRow _result)
              (CallFunction|SearchTalkData))))))))

(event EventBeginPlay
  (bind _returnvalue (UserInterface|CreateWidget "/Game/TPSprite/Blueprints/WBP_ActionGuide.WBP_ActionGuide_C"))
  (UserInterface|Viewport|AddtoViewport _returnvalue 0)
  (bind _output_get (Variables|Default|SetActionGuide _returnvalue))
  (Widget|SetVisibility _output_get "Hidden"))

(event Collision|EventActorBeginOverlap
  (params (OtherActor :type Actor%20Object%20Reference)))

(event EventBPITalkEnd
  (params (WBP_Talk :type WBP%20Talk%20Object%20Reference) (EndTalk :type Boolean) (NPC :type BP%20NPC%20Belt%20Object%20Reference) (SetFlag :type E_Flag_MainEvent%20Enum :default "NewEnumerator3")))

(event EventTick
  (params (DeltaSeconds :type Float%20%28single-precision%29)))

(event EventBPITalkStart
  (params (WBP_Talk :type WBP%20Talk%20Object%20Reference) (EndTalk :type Boolean) (NameText :type String) (TalkText :type Array%20of%20Strings) (NPC :type BP%20NPC%20Belt%20Object%20Reference) (RequiredFlag :type E_Flag_MainEvent%20Enum :default "NewEnumerator0") (SetFlag :type E_Flag_MainEvent%20Enum :default "NewEnumerator0"))
  (Variables|Default|SetWBP%20Talk WBP_Talk)
  (Variables|Default|SetSearch_TalkRow (Variables|Default|GetSearch_TalkRow))
  (CallFunction|SearchTalkData))

(fn ConstructionScript)